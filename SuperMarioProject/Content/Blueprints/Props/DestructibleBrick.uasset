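; A destructible brick prop that shatters the first time its OnPlayerHit event fires, then destroys itself after a short delay.
; The hit hides the intact cube and disables its collision, then reveals the GCDestructibleBrick component with physics simulation turned on.
; An FS_MasterField actor is spawned at the hit location and triggered to act on the revealed brick.
; A flag limits the break to one hit.
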(event `self.ReceiveBeginPlay`
  (add `self.OnPlayerHit` (delegate `OnPlayerHit_Event`)))

(event `OnPlayerHit_Event` :!signature `self.OnPlayerHit`
  (params (HitLocation :type "Vector Structure"))
  (`KismetSystemLibrary.PrintString` "Hello")
  (if (not (`self.IsPlayerPreviouslyHit`))
    (`self.HideCube`)
    (`self.ShowDestructibleBrick` HitLocation)
    (set `self.IsPlayerPreviouslyHit` true)))

(event `HideCube`
  (bind _cube (`self.Cube`))
  (`SceneComponent.SetVisibility` _cube false true)
  (`SceneComponent.SetHiddenInGame` _cube true false)
  (`PrimitiveComponent.SetCollisionResponseToAllChannels` _cube "ECR_Ignore"))

(event `ShowDestructibleBrick`
  (params (HitLocation :type "Vector Structure"))
  (bind _gc_destructiblebrick (`self.GC_DestructibleBrick`))
  (`SceneComponent.SetVisibility` _gc_destructiblebrick true true)
  (`SceneComponent.SetHiddenInGame` _gc_destructiblebrick false false)
  (`PrimitiveComponent.SetSimulatePhysics` _gc_destructiblebrick true)
  (bind _returnvalue (`|SpawnActorFromClass` "/Engine/EditorResources/FieldNodes/FS_MasterField.FS_MasterField_C" (`KismetMathLibrary.Conv_VectorToTransform` HitLocation) "Undefined" "MultiplyWithRoot" null null))
  (set `/Engine/EditorResources/FieldNodes/FS_MasterField.ActivationType` "NewEnumerator4" _returnvalue)
  (`/Engine/EditorResources/FieldNodes/FS_MasterField.CE_Trigger` _returnvalue)
  (`KismetSystemLibrary.Delay` 2.0)
  (`self.K2_DestroyActor`))

(fn `UserConstructionScript`)